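; Player character Blueprint that moves in discrete hops along four world-axis directions.
; Releasing a MoveForward, MoveBack, MoveLeft or MoveRight action calls Jump, instantly offsets the capsule by a fixed step, and turns the Scene component to face that direction.
; Pressing any of these actions calls StopJumping.
; The offset is unswept, so each step ignores blocking collision along its path.
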(event EventBeginPlay)

(event Collision|EventActorBeginOverlap
  (params (OtherActor :type Actor%20Object%20Reference)))

(event EventTick
  (params (DeltaSeconds :type Float%20%28single-precision%29)))

(event Input|ActionEvents|InputActionMoveRight
  (params (Key :type Key%20Structure :default "None"))
  (:Pressed
    (Character|StopJumping))
  (:Released
    (Character|Jump)
    (Transformation|AddWorldOffset (Variables|Collision|GetCapsuleComponent) "0,100.000000, 0" false false)
    (Transformation|SetWorldRotation (Variables|Default|GetScene) "0,90.000000, 0" false false)))

(event Input|ActionEvents|InputActionMoveLeft
  (params (Key :type Key%20Structure :default "None"))
  (:Pressed
    (Character|StopJumping))
  (:Released
    (Character|Jump)
    (Transformation|SetWorldRotation (Variables|Default|GetScene) "0,-90.000000, 0" false false)
    (Transformation|AddWorldOffset (Variables|Collision|GetCapsuleComponent) "0,-100.000000,0.000000" false false)))

(event Input|ActionEvents|InputActionMoveBack
  (params (Key :type Key%20Structure :default "None"))
  (:Pressed
    (Character|StopJumping))
  (:Released
    (Character|Jump)
    (Transformation|SetWorldRotation (Variables|Default|GetScene) "0,180.000000,0.000000" false false)
    (Transformation|AddWorldOffset (Variables|Collision|GetCapsuleComponent) "-100.000000, 0, 0" false false)))

(event Input|ActionEvents|InputActionMoveForward
  (params (Key :type Key%20Structure :default "None"))
  (:Pressed
    (Character|StopJumping))
  (:Released
    (Character|Jump)
    (Transformation|AddWorldOffset (Variables|Collision|GetCapsuleComponent) "100.000000, 0, 0" false false)
    (Transformation|SetWorldRotation (Variables|Default|GetScene) "0, 0,0.000000" false false)))

(fn ConstructionScript)