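; Level manager for a Crossy Road-style game that scrolls along world X and detects actors reaching its bounds.
; Every tick it offsets its root by GM_CrossyRoad's GameSpeed, without delta-time scaling.
; Actors entering the LevelBounds box are asked for their parent via ReturnParentMessage, which is then notified through SpawnActorHitBounds.
; The construction script sizes and places that box from the out-of-bounds variables.
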(event OnComponentBeginOverlap(LevelBounds)
  (params (OverlappedComponent :type Primitive%20Component%20Object%20Reference) (OtherActor :type Actor%20Object%20Reference) (OtherComp :type Primitive%20Component%20Object%20Reference) (OtherBodyIndex :type Integer) (bFromSweep :type Boolean) (SweepResult :type Hit%20Result%20Structure%20%28by%20ref%29))
  (bind _parent (Class|BPISpawner|ReturnParent(Message) OtherActor))
  (Utilities|IsValid _parent
    (:Is%20Valid
      (Default|SpawnActorHitBounds _parent OtherActor))))

(event EventBeginPlay)

(event Collision|EventActorBeginOverlap
  (params (OtherActor :type Actor%20Object%20Reference)))

(event EventTick
  (params (DeltaSeconds :type Float%20%28single-precision%29))
  (bind _asgm_crossy_road (Utilities|Casting|CastToGM_CrossyRoad (Game|GetGameMode)))
  (Transformation|AddWorldOffset (Variables|Default|GetDefaultSceneRoot) (Math|Vector|MakeVector (Variables|/Game/Blueprints/GM_CrossyRoad.GM_CrossyRoad_C|GetGameSpeed _asgm_crossy_road) 0.0 0.0) false false))

(fn ConstructionScript
  (bind _levelbounds (Variables|Default|GetLevelBounds))
  (Components|Box|SetBoxExtent _levelbounds (Variables|Default|GetOutOfBoundsScale) true)
  (Transformation|SetWorldLocation _levelbounds (Variables|Default|GetOutOfBoundsLocation) false false))