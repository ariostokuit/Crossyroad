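; Game mode for a Crossy Road-style game that tracks score, coins, game speed and game-over state.
; On BeginPlay it makes the BP_LevelManager tagged MainCamera the player's view target, creates the HUD and calls Reset.
; Score and coin update events clamp totals at zero and push them to the HUD.
; Reset restores score, speed and world bounds but leaves coins untouched, while GameOver sets the flag and zeroes GameSpeed.
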(event Custom|Reset
  ;[1 1 1] Reset Game
  (Variables|Default|SetCurrentScore 0)
  (Variables|/Game/Blueprints/UI/Game_HUD.Game_HUD_C|SetScore (Variables|Default|GetHUD) 0)
  (Variables|Default|SetisGameOver false)
  (Variables|Default|SetGameSpeed 1.0)
  (Variables|Default|SetWorldBounds 3e+03))

(event Custom|Game%20Over
  ;[1 1 1] Death Screen
  (Variables|Default|SetisGameOver true)
  (Variables|Default|SetGameSpeed 0.0))

(event Custom|UpdateCoin
  (params (Coins :type Integer))
  ;[1 1 1] Updates Coins
  (if (<= (+ Coins (Variables|Default|GetCurrentCoins)) 0)
    (Variables|Default|SetCurrentCoins 0)
    (else
      (Variables|Default|SetCurrentCoins (+ Coins (Variables|Default|GetCurrentCoins)))))
  (Variables|/Game/Blueprints/UI/Game_HUD.Game_HUD_C|SetCoins (Variables|Default|GetHUD) (Variables|Default|GetCurrentCoins)))

(event Custom|UpdateScore
  (params (Points :type Integer))
  ;[1 1 1] Updates Score
  (if (<= (+ Points (Variables|Default|GetCurrentScore)) 0)
    (Variables|Default|SetCurrentScore 0)
    (else
      (Variables|Default|SetCurrentScore (+ Points (Variables|Default|GetCurrentScore)))))
  (Variables|/Game/Blueprints/UI/Game_HUD.Game_HUD_C|SetScore (Variables|Default|GetHUD) (Variables|Default|GetCurrentScore)))

(event EventBeginPlay
  (bind _outactors (Actor|GetAllActorsOfClass "/Game/Blueprints/BP_LevelManager.BP_LevelManager_C"))
  (for _array_element _outactors
    (if (Actor|ActorHasTag _array_element "MainCamera")
      (bind _output_get (Variables|Default|SetLevelManager _array_element))
      (Game|Player|SetViewTargetwithBlend (Game|GetPlayerController 0) _output_get 0.0 "VTBlend_Linear" 0.0 false)
      (bind _returnvalue (UserInterface|CreateWidget "/Game/Blueprints/UI/Game_HUD.Game_HUD_C"))
      (bind _output_get_2 (Variables|Default|SetHUD _returnvalue))
      (UserInterface|Viewport|AddtoViewport _output_get_2 0)
      (CallFunction|Reset))))

(fn ConstructionScript)