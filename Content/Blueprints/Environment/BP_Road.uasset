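; BP_Road is an environment road actor that spawns random vehicles at one of its two ends.
; On BeginPlay it randomly picks the east or west spawn point and stores that transform.
; Each Tick spawns a random class from VehicleClasses there and appends it to the Vehicles array, with no timer gate or count limit in the graph.
; Direction and destroy nodes are left unconnected.
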(event EventBeginPlay
  (|CallParentFunction)
  (if (Math|Random|RandomBool)
    (Variables|Default|SetSpawnTransform (Transformation|GetWorldTransform (Variables|Default|GetSpawnEast)))
    (else
      (Variables|Default|SetSpawnTransform (Transformation|GetWorldTransform (Variables|Default|GetSpawnWest))))))

(event Collision|EventActorBeginOverlap
  (params (OtherActor :type Actor%20Object%20Reference))
  (|CallParentFunction OtherActor) ; This node is disabled and will not be called.\nDrag off pins to build functionality.
)

(event EventTick
  (params (DeltaSeconds :type Float%20%28single-precision%29))
  (bind _vehicleclasses (Variables|Default|GetVehicleClasses))
  (|CallParentFunction DeltaSeconds)
  (bind _returnvalue (Game|SpawnActorfromClass (Utilities|Array|Get(acopy) _vehicleclasses (Math|Random|RandomInteger (Utilities|Array|Length _vehicleclasses))) (Variables|Default|GetSpawnTransform) "Undefined" 0 0))
  (Utilities|Array|Add (Variables|Default|GetVehicles) _returnvalue))

(fn ConstructionScript
  (|CallParentFunction))