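; BP_Floor_River is a river floor segment that continuously spawns moving river objects, such as logs, from a randomly chosen side.
; On BeginPlay it rolls one speed for the segment, derives the spawn interval range from it, and picks the east or west spawn point.
; A self-rescheduling timer spawns a random RiverClasses actor there and passes it that speed.
; Slower segments get longer gaps between spawns, faster ones shorter gaps.
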(event Custom|SpawnVehicle
  (bind _riverclasses (Variables|Default|GetRiverClasses))
  (bind _returnvalue (Game|SpawnActorfromClass (Utilities|Array|Get(acopy) _riverclasses (Math|Random|RandomInteger (Utilities|Array|Length _riverclasses))) (Transformation|GetWorldTransform (Variables|Default|GetSpawnPoint)) "AlwaysSpawn" 0 0))
  (Variables|/Game/Blueprints/Entities/vehicle_assets/BP_vehicle.BP_Vehicle_C|SetSpeed _returnvalue (Variables|Default|GetSpeedOfLogs))
  (Utilities|Time|SetTimerbyEvent (delegate Custom|SpawnVehicle) (Math|Random|RandomFloatinRange (Variables|Default|GetMinFrequency) (Variables|Default|GetMaxFrequency))))

(event EventBeginPlay
  (|CallParentFunction)
  (bind _output_get (Variables|Default|SetSpeedOfLogs (Math|Random|RandomFloatinRange 2.0 5.0)))
  (if (< _output_get 4.0)
    (Variables|Default|SetMinFrequency 2.8)
    (Variables|Default|SetMaxFrequency 4.5)
    (else
      (Variables|Default|SetMinFrequency 1.0)
      (Variables|Default|SetMaxFrequency 2.0)))
  (if (Math|Random|RandomBool)
    (Variables|Default|SetSpawnPoint (Variables|Default|GetSpawnEast))
    (else
      (Variables|Default|SetSpawnPoint (Variables|Default|GetSpawnWest))))
  (Utilities|Time|SetTimerbyEvent (delegate Custom|SpawnVehicle) (Math|Random|RandomFloatinRange 1.0 2.0)))

(fn ConstructionScript
  (|CallParentFunction))