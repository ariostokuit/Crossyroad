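; Floor spawner, built on a parent spawner, that maintains an endless strip of floor tiles along X.
; On BeginPlay it lays out the starting row, measuring tile length from the first tile's bounds and chaining each new tile off the forward-most one.
; When a tile hits the bounds, it is destroyed and a replacement is appended at the front.
; An alternator switches between two floor pools, with a random pick within each.
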(event EventBeginPlay
  (|CallParentFunction)
  (for _index (range 0 (Variables|Default|GetFloorsRequired))
    (bind _isa (Utilities|FlowControl|FlipFlop)
      (:A
        _)
      (:B
        _))
    (bind _output_get (Variables|Default|SetAlternator _isa))
    (bind _output (CallFunction|GetRandomFloor _output_get))
    (if (== _index 0)
      (bind _returnvalue (CallFunction|SpawnActor _output))
      (Variables|Default|SetForwardFloor _returnvalue)
      (Variables|Default|SetFloorSize (* (.x (.BoxExtent (Collision|GetActorBounds _returnvalue false))) 2.0))
      (Transformation|SetActorLocation (Variables|Default|GetForwardFloor) (Transformation|GetActorLocation) false false)
      (else
        (bind _returnvalue_2 (CallFunction|SpawnActor _output))
        (Transformation|SetActorLocation _returnvalue_2 (Math|Vector|MakeVector (+ (.x (Transformation|GetActorLocation (Variables|Default|GetForwardFloor))) (Variables|Default|GetFloorSize)) (.y (Transformation|GetActorLocation (Variables|Default|GetForwardFloor))) 0.0) false false)
        (Variables|Default|SetForwardFloor _returnvalue_2)))))

(fn ConstructionScript
  (|CallParentFunction))

(fn SpawnActor
  (params (SpawnActorType :type Actor%20Class%20Reference))
  (bind _returnvalue (|CallParentFunction SpawnActorType))
  (return _returnvalue))

(fn SpawnActorHitBounds
  (params (OutOfBoundsActor :type Actor%20Object%20Reference))
  (|CallParentFunction OutOfBoundsActor)
  (Actor|DestroyActor OutOfBoundsActor)
  (bind _output_get (Variables|Default|SetAlternator (not (Variables|Default|GetAlternator))))
  (bind _output (CallFunction|GetRandomFloor _output_get))
  (bind _returnvalue (CallFunction|SpawnActor _output))
  (Transformation|SetActorLocation _returnvalue (Math|Vector|MakeVector (+ (.x (Transformation|GetActorLocation (Variables|Default|GetForwardFloor))) (Variables|Default|GetFloorSize)) (.y (Transformation|GetActorLocation (Variables|Default|GetForwardFloor))) 0.0) false false)
  (Variables|Default|SetForwardFloor _returnvalue))

(fn GetRandomFloor
  (params (Alternator :type Boolean))
  (if Alternator
    (return (Utilities|Array|Get(acopy) (Variables|Default|GetFloorTypes_0) (Math|Random|RandomIntegerinRange 0 2)))
    (else
      (return (Utilities|Array|Get(acopy) (Variables|Default|GetFloorTypes_1) (Math|Random|RandomIntegerinRange 0 2))))))