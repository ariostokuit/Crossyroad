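; BP_Floor_Road is a road floor piece that continuously spawns moving vehicles from one side.
; On BeginPlay it rolls a shared vehicle speed and randomly picks the east or west spawn point, both fixed for that road's lifetime.
; A timer re-armed with a random delay after each spawn creates a random class from VehicleClasses at that point and passes it the road's speed.
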(event Custom|SpawnVehicle
  (bind _vehicleclasses (Variables|Default|GetVehicleClasses))
  (bind _returnvalue (Game|SpawnActorfromClass (Utilities|Array|Get(acopy) _vehicleclasses (Math|Random|RandomInteger (Utilities|Array|Length _vehicleclasses))) (Transformation|GetWorldTransform (Variables|Default|GetSpawnPoint)) "Undefined" 0 0))
  (Variables|/Game/Blueprints/Entities/vehicle_assets/BP_vehicle.BP_Vehicle_C|SetSpeed _returnvalue (Variables|Default|GetSpeedOfVehicles))
  (Utilities|Time|SetTimerbyEvent (delegate Custom|SpawnVehicle) (Math|Random|RandomFloatinRange 0.6 5.0)))

(event EventBeginPlay
  (|CallParentFunction)
  (Variables|Default|SetSpeedOfVehicles (Math|Random|RandomFloatinRange 4.0 6.0))
  (if (Math|Random|RandomBool)
    (Variables|Default|SetSpawnPoint (Variables|Default|GetSpawnEast))
    (else
      (Variables|Default|SetSpawnPoint (Variables|Default|GetSpawnWest))))
  (Utilities|Time|SetTimerbyEvent (delegate Custom|SpawnVehicle) (Math|Random|RandomFloatinRange 0.6 5.0)))

(event EventTick
  (params (DeltaSeconds :type Float%20%28single-precision%29))
  (|CallParentFunction DeltaSeconds))

(fn ConstructionScript
  (|CallParentFunction))