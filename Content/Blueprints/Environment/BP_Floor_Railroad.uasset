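; Railroad floor tile that sends a train across when the player enters its trigger.
; BeginPlay picks a random train speed and an east or west spawn point, both fixed for that tile.
; After a random short delay, a timer lights the warning spotlight and plays a sound, then turns the light off and spawns BP_Vehicle_Train.
; A flag blocks retriggering until a random cooldown after the spawn ends.
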(event OnComponentBeginOverlap(Trigger)
  (params (OverlappedComponent :type Primitive%20Component%20Object%20Reference) (OtherActor :type Actor%20Object%20Reference) (OtherComp :type Primitive%20Component%20Object%20Reference) (OtherBodyIndex :type Integer) (bFromSweep :type Boolean) (SweepResult :type Hit%20Result%20Structure%20%28by%20ref%29))
  (if (and (not (Variables|Default|GetIsTrainWarningOn)) (== OtherActor (Game|Player|GetPlayerPawn 0)))
    (Variables|Default|SetIsTrainWarningOn true)
    (Utilities|Time|SetTimerbyEvent (delegate Custom|Train%20Warning) (Math|Random|RandomFloatinRange 0.0 2.5))))

(event Custom|Train%20Warning
  (bind _spotlight (Variables|Default|GetSpotLight))
  (Rendering|ToggleVisibility _spotlight false)
  (Audio|SpawnSoundAttached "/Game/Blueprints/Audio/TrainSound_Cue.TrainSound_Cue" (Variables|Default|GetWarningSign) "None" "0, 0, 0" "0, 0, 0" "KeepRelativeOffset" false 1.0 1.0 0.0 0 0)
  (Utilities|FlowControl|Delay 1.5)
  (Rendering|ToggleVisibility _spotlight false)
  (CallFunction|SpawnTrain)
  ;[1 1 1] Delay before being able to be triggered again
  (Utilities|FlowControl|Delay (Math|Random|RandomFloatinRange 2.0 4.0))
  (Variables|Default|SetIsTrainWarningOn false))

(event Custom|Spawn%20Train
  ;[1 1 1] Spawns Train
  (bind _returnvalue (Game|SpawnActorfromClass "/Game/Blueprints/Entities/vehicle_assets/BP_Vehicle_Train.BP_Vehicle_Train_C" (Transformation|GetWorldTransform (Variables|Default|GetSpawnPoint)) "Undefined" 0 0))
  (Variables|/Game/Blueprints/Entities/vehicle_assets/BP_vehicle.BP_Vehicle_C|SetSpeed _returnvalue (Variables|Default|GetSpeedOfTrain)))

(event EventBeginPlay
  (|CallParentFunction)
  (Variables|Default|SetFloorSize (.x (.BoxExtent (Collision|GetComponentBounds (Variables|Default|GetFloorMesh_0)))))
  (Rendering|SetVisibility (Variables|Default|GetSpotLight) false false)
  (Variables|Default|SetSpeedOfTrain (Math|Random|RandomFloatinRange 35.0 5e+01))
  (if (Math|Random|RandomBool)
    (Variables|Default|SetSpawnPoint (Variables|Default|GetSpawnEast))
    (else
      (Variables|Default|SetSpawnPoint (Variables|Default|GetSpawnWest)))))

(event Collision|EventActorBeginOverlap
  (params (OtherActor :type Actor%20Object%20Reference)))

(event EventTick
  (params (DeltaSeconds :type Float%20%28single-precision%29)))

(fn ConstructionScript
  (|CallParentFunction))