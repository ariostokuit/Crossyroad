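; Environment spawner that continuously spawns random actors from a list of river classes at one side of its lane.
; On BeginPlay it randomly chooses the east or west spawn point and keeps that side for its lifetime.
; A timer fires SpawnVehicle, which spawns a random class at that point, then re-arms itself with a fresh random delay of a few seconds, forming an endless, irregular loop.
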(event Custom|SpawnVehicle
  (bind _riverclasses (Variables|Default|GetRiverClasses))
  (Game|SpawnActorfromClass (Utilities|Array|Get(acopy) _riverclasses (Math|Random|RandomInteger (Utilities|Array|Length _riverclasses))) (Transformation|GetWorldTransform (Variables|Default|GetSpawnPoint)) "Undefined" 0 0)
  (Utilities|Time|SetTimerbyEvent (delegate Custom|SpawnVehicle) (Math|Random|RandomFloatinRange 2.0 5.0)))

(event EventBeginPlay
  (|CallParentFunction)
  (if (Math|Random|RandomBool)
    (Variables|Default|SetSpawnPoint (Variables|Default|GetSpawnEast))
    (else
      (Variables|Default|SetSpawnPoint (Variables|Default|GetSpawnWest))))
  (Utilities|Time|SetTimerbyEvent (delegate Custom|SpawnVehicle) (Math|Random|RandomFloatinRange 2.0 5.0)))

(fn ConstructionScript
  (|CallParentFunction))